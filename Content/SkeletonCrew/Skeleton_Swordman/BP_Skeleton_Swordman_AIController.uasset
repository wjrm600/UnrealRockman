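; AI controller for the Skeleton Swordman enemy that runs its behavior tree on possession.
; AI perception stores a sensed Player-tagged actor and line of sight in the Blackboard.
; Other perception updates, including losing the player, start a timer that clears both when it expires.
; Separate events copy the pawn's attack, damage and death flags into the Blackboard.
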(event `self.ReceivePossess`
  (params (PossessedPawn :type "Pawn Object Reference"))
  (`self.RunBehaviorTree` "/Game/SkeletonCrew/Skeleton_Swordman/Skeleton_Swordman_BehaviorTree.Skeleton_Swordman_BehaviorTree"))

(event `self.ReceiveBeginPlay`)

(event `self.AIPerception.OnTargetPerceptionUpdated`
  (params (Actor :type "Actor Object Reference") (Stimulus :type "AIStimulus Structure"))
  (bind _blackboard (`self.Blackboard`))
  (`|ExecutionSequence`
    (:`then_0`
      (if true
        _))
    (:`then_1`
      (if (and (`self.ActorHasTag` Actor "Player") (`.bSuccessfullySensed` (break `AIStimulus` Stimulus)))
        (`KismetSystemLibrary.K2_ClearAndInvalidateTimerHandle` (`self.Enemy_Timer`))
        (`BlackboardComponent.SetValueAsBool` _blackboard (`self.Has_Line_Of_Sight`) true)
        (`BlackboardComponent.SetValueAsObject` _blackboard (`self.Enemy_Actor`) Actor)
        (else
          (bind _returnvalue (`KismetSystemLibrary.K2_SetTimerDelegate` (delegate `StartEnemyTimer`) (`self.Line_Of_Sight_Timer`)))
          (set `self.Enemy_Timer` _returnvalue))))))

(event `StartEnemyTimer`
  (bind _blackboard (`self.Blackboard`))
  (`BlackboardComponent.SetValueAsBool` _blackboard (`self.Has_Line_Of_Sight`) false)
  (`BlackboardComponent.SetValueAsObject` _blackboard (`self.Enemy_Actor`) null))

(event `AICon_BlackBoard_SetIsAttack`
  (bind _asskeleton_swordman (cast `/Game/SkeletonCrew/Skeleton_Swordman/Skeleton_Swordman` (`self.K2_GetPawn`)))
  (`BlackboardComponent.SetValueAsBool` (`self.Blackboard`) (`self.IsAttack`) (`/Game/SkeletonCrew/Skeleton_Swordman/Skeleton_Swordman.IsAttack` _asskeleton_swordman)))

(event `AICon_BlackBoard_SetIsDamage`
  (bind _asskeleton_swordman (cast `/Game/SkeletonCrew/Skeleton_Swordman/Skeleton_Swordman` (`self.K2_GetPawn`)))
  (`BlackboardComponent.SetValueAsBool` (`self.Blackboard`) (`self.IsDamage`) (`/Game/SkeletonCrew/Skeleton_Swordman/Skeleton_Swordman.IsDamage` _asskeleton_swordman)))

(event `AnyDama`
  (bind _asskeleton_swordman (cast `/Game/SkeletonCrew/Skeleton_Swordman/Skeleton_Swordman` (`self.K2_GetPawn`)))
  (`BlackboardComponent.SetValueAsBool` (`self.Blackboard`) (`self.IsDead`) (`/Game/SkeletonCrew/Skeleton_Swordman/Skeleton_Swordman.IsDead` _asskeleton_swordman)))

(fn `BP_Skeleton_Swordman_AIController_AutoGenFunc`
  (params (DamagedActor :type "Actor Object Reference") (Damage :type "Float (double-precision)") (DamageType :type "DamageType Object Reference") (InstigatedBy :type "Controller Object Reference") (DamageCauser :type "Actor Object Reference")))

(fn `UserConstructionScript`)